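; Ice attack projectile actor that is aimed with the mouse cursor and launched on left click.
; Until launched, Tick turns its yaw toward the cursor hit point and holds the MagicCircle at the cursor hit height captured on BeginPlay.
; Left click hides the circle, sets a flat velocity along ForwardDirection at max speed, and enables ProjectileMovement simulation, which also stops the aiming.
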(event `self.ReceiveBeginPlay`
  (set `self.MouseLocation` (`.Location` (`GameplayStatics.BreakHitResult` (`PlayerController.GetHitResultUnderCursorByChannel` (`GameplayStatics.GetPlayerController` 0) "TraceTypeQuery1" true)))))

(event `Key|LeftMouseButton`
  (params (Key :type "Key Structure"))
  (bind _projectilemovement (`self.ProjectileMovement`))
  (bind _returnvalue (`MovementComponent.GetMaxSpeed` _projectilemovement))
  (:`Pressed`
    (set `MovementComponent.Velocity` (* (`SceneComponent.GetForwardVector` (`self.ForwardDirection`)) (`KismetMathLibrary.MakeVector` _returnvalue _returnvalue)) _projectilemovement)
    (`SceneComponent.SetVisibility` (`self.MagicCircle`) false false)
    (set `ProjectileMovementComponent.bSimulationEnabled` true _projectilemovement)))

(event `self.ReceiveTick`
  (params (DeltaSeconds :type "Float (single-precision)"))
  (bind (_returnvalue_roll _returnvalue_pitch) (`KismetMathLibrary.BreakRotator` (`self.K2_GetActorRotation`)))
  (bind _magiccircle (`self.MagicCircle`))
  (bind (_mouselocation_x _mouselocation_y _mouselocation_z) (`KismetMathLibrary.BreakVector` (`self.MouseLocation`)))
  (bind (_returnvalue_x _returnvalue_y) (`KismetMathLibrary.BreakVector` (`SceneComponent.K2_GetComponentLocation` _magiccircle)))
  (bind (_returnvalue_roll_2 _returnvalue_pitch_2 _returnvalue_yaw) (`KismetMathLibrary.BreakRotator` (`KismetMathLibrary.FindLookAtRotation` (`self.K2_GetActorLocation`) (`.Location` (`GameplayStatics.BreakHitResult` (`PlayerController.GetHitResultUnderCursorByChannel` (`GameplayStatics.GetPlayerController` 0) "TraceTypeQuery1" true))))))
  (if (not (`ProjectileMovementComponent.bSimulationEnabled` (`self.ProjectileMovement`)))
    (`self.K2_SetActorRotation` (`KismetMathLibrary.MakeRotator` _returnvalue_roll _returnvalue_pitch _returnvalue_yaw))
    (`SceneComponent.K2_SetWorldLocation` _magiccircle (`KismetMathLibrary.MakeVector` _returnvalue_x _returnvalue_y _mouselocation_z) false true)))

(fn `UserConstructionScript`
  (`parent.UserConstructionScript`))